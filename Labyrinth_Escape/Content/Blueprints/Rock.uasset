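; Rock is a pickup actor the player collects by pressing Interact while standing inside its InteractionCollision.
; It enables input for player controller 0 on BeginPlay.
; Overlap begin and end with BP_ThirdPersonCharacter open and close a gate on the input event.
; A successful press increments that character's RockAmount and destroys the rock.
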(event OnComponentBeginOverlap(InteractionCollision)
  (params (OverlappedComponent :type Primitive%20Component%20Object%20Reference) (OtherActor :type Actor%20Object%20Reference) (OtherComp :type Primitive%20Component%20Object%20Reference) (OtherBodyIndex :type Integer) (bFromSweep :type Boolean) (SweepResult :type Hit%20Result%20Structure%20%28by%20ref%29))
  ;[0.3422 0.8799 1] Detecting overlapping with InteractionCollision and if the player has pressed InputAction F when it's overlapping.
  (bind _asbp_third_person_character (Utilities|Casting|CastToBP_ThirdPersonCharacter OtherActor))
  (Utilities|FlowControl|Gate true) ; enters at Open
)

(event OnComponentEndOverlap(InteractionCollision)
  (params (OverlappedComponent :type Primitive%20Component%20Object%20Reference) (OtherActor :type Actor%20Object%20Reference) (OtherComp :type Primitive%20Component%20Object%20Reference) (OtherBodyIndex :type Integer))
  ;[0.3422 0.8799 1] Detecting overlapping with InteractionCollision and if the player has pressed InputAction F when it's overlapping.
  (Utilities|Casting|CastToBP_ThirdPersonCharacter OtherActor)
  (Utilities|FlowControl|Gate true) ; enters at Close
)

(event EventBeginPlay
  (Input|EnableInput (Game|GetPlayerController 0)))

(event Input|ActionEvents|InputActionInteract
  (params (Key :type Key%20Structure :default "None"))
  ;[0.3422 0.8799 1] Detecting overlapping with InteractionCollision and if the player has pressed InputAction F when it's overlapping.
  (:Pressed
    (Utilities|FlowControl|Gate true
      (:Exit
        (bind _result (Math|Integer|IncrementInt (Variables|/Game/Blueprints/BP_ThirdPersonCharacter.BP_ThirdPersonCharacter_C|GetRock%20Amount (stale OnComponentBeginOverlap(InteractionCollision) _asbp_third_person_character)))
          (:%20%20
            (Variables|/Game/Blueprints/BP_ThirdPersonCharacter.BP_ThirdPersonCharacter_C|SetRock%20Amount (stale OnComponentBeginOverlap(InteractionCollision) _asbp_third_person_character) _result)
            (Actor|DestroyActor)))))))

(fn ConstructionScript)